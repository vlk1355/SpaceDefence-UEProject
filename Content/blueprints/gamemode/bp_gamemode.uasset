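; Wave-based game mode that spawns growing waves of BP_Enemy aliens, starting shortly after BeginPlay.
; Each new wave increments the wave counter, scales difficulty and alien count by a multiplier, and starts a looping timer.
; The timer spawns aliens at random TargetPoints, tracking them in AlienList until the count runs out.
; RegisterAlienDeath removes aliens from the list and, once none remain alive or pending, triggers the next wave after a delay.
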(event `self.ReceiveBeginPlay`
  (`KismetSystemLibrary.Delay` 3.0)
  (`self.Set Up New Wave`))

(event `waveSpawn`
  (`self.spawnAlien`))

(event `waveEnd`
  (`KismetSystemLibrary.Delay` 2.0)
  (`self.Set Up New Wave`))

(fn `getRandomSpawnPoint`
  (returns (Output :type "TargetPoint Object Reference"))
  (bind _outactors (`GameplayStatics.GetAllActorsOfClass` "/Script/Engine.TargetPoint"))
  (return (`|GetArrayItem` _outactors (`KismetMathLibrary.RandomIntegerInRange` 0 (`KismetArrayLibrary.Array_LastIndex` _outactors)))))

(fn `increseDiff`
  (bind _returnvalue (`KismetMathLibrary.Round` (* (`self.waveDiff`) (`self.diffMult`))))
  (set `self.waveDiff` _returnvalue)
  (set `self.alienCount` _returnvalue))

(fn `Register alien Death`
  (params (Alien :type "/Game/blueprints/AI/BP_Enemy Object Reference (by ref)"))
  (`KismetArrayLibrary.Array_RemoveItem` (`self.AlienList`) Alien)
  (if (`self.waveClearCheck`)
    (`self.waveEnd`)))

(fn `Set Up New Wave`
  (bind _result (`/Engine/EditorBlueprintResources/StandardMacros.IncrementInt` (`self.curentWawe`))
    (:`  `
      (set `self.curentWawe` _result)
      (`self.increseDiff`)
      (`KismetSystemLibrary.K2_SetTimer` null "waveSpawn" 1.0 true))))

(fn `spawnAlien`
  (bind _output (`self.getRandomSpawnPoint`))
  (`/Engine/EditorBlueprintResources/StandardMacros.IsValid` _output
    (:`Is Valid`
      (bind _returnvalue (`|SpawnActorFromClass` "/Game/blueprints/AI/BP_Enemy.BP_Enemy_C" (`self.GetTransform` _output) "Undefined" "OverrideRootScale" null null))
      (`/Engine/EditorBlueprintResources/StandardMacros.IsValid` _returnvalue
        (:`Is Valid`
          (`KismetArrayLibrary.Array_Add` (`self.AlienList`) _returnvalue)
          (bind _result (`/Engine/EditorBlueprintResources/StandardMacros.DecrementInt` (`self.alienCount`))
            (:`  `
              (if (== _result 0)
                (`KismetSystemLibrary.K2_ClearTimer` null "waveSpawn")))))))))

(fn `UserConstructionScript`)

(fn `waveClearCheck`
  (returns (ReturnValue :type Boolean))
  (return (and (== (`KismetArrayLibrary.Array_Length` (`self.AlienList`)) 0) (== (`self.alienCount`) 0))))